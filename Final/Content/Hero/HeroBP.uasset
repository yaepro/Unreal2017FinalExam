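; Player hero character with world-axis movement, a gun and melee punching.
; It spawns a gun onto a mesh socket at BeginPlay, fires it while left mouse is held, and toggles hand-socket collision spheres for punches.
; Both movement axes share a once-per-tick rotation gate that derives facing from MoveForward alone.
; Clicks move MouseClickPoint to the cursor hit, but its spawn and cursor-display setup are disconnected.
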(event `self.ReceiveBeginPlay`
  (bind _returnvalue (`|SpawnActorFromClass` "/Game/Gun/GunBP.GunBP_C" (`SceneComponent.K2_GetComponentToWorld` (`self.Mesh`)) "Undefined" "OverrideRootScale"))
  (bind _output_get (set `self.Gun` _returnvalue))
  (`self.K2_AttachToComponent` _output_get (`self.Mesh`) "GunSocket" "SnapToTarget" "SnapToTarget" "KeepRelative" true))

(event `InputAxis|MoveForward`
  (params (AxisValue :type "Float (single-precision)"))
  (`self.AddMovementInput` (1.0 0.0 0.0) AxisValue)
  (`/Engine/EditorBlueprintResources/StandardMacros.DoOnce` false :!label _label
    (:`Completed`
      (`KismetSystemLibrary.Delay` 0.0)
      (`self.K2_SetActorRotation` (`KismetMathLibrary.Conv_VectorToRotator` (`KismetMathLibrary.MakeVector` AxisValue (stale `InputAxis|MoveRight` AxisValue))))
      (goto _label :!via `Reset`))))

(event `InputAction|LeftMouseClicked`
  (params (Key :type "Key Structure" :default "AnyKey"))
  (bind _gun (`self.Gun`))
  (:`Pressed`
    (`/Game/Gun/GunBP.StartFiring` _gun)
    (`self.K2_SetActorLocation` (`self.MouseClickPoint`) (`.Location` (`GameplayStatics.BreakHitResult` (`PlayerController.GetHitResultUnderCursorByChannel` (`GameplayStatics.GetPlayerController` 0) "TraceTypeQuery1" true))) false false :!label _label_2))
  (:`Released`
    (`/Game/Gun/GunBP.StopFiring` _gun)
    (goto _label_2)))

(event `InputAxis|MoveRight`
  (params (AxisValue :type "Float (single-precision)"))
  (`self.AddMovementInput` (0.0 1.0 0.0) AxisValue)
  (goto _label))

(event `StartPunching`
  (set `self.IsPuncing` true)
  (`PrimitiveComponent.SetCollisionEnabled` (`self.LHandSphere`) "QueryOnly")
  (`PrimitiveComponent.SetCollisionEnabled` (`self.RHandSphere`) "QueryOnly"))

(event `StopPunching`
  (set `self.IsPuncing` false)
  (`PrimitiveComponent.SetCollisionEnabled` (`self.LHandSphere`) "NoCollision")
  (`PrimitiveComponent.SetCollisionEnabled` (`self.RHandSphere`) "NoCollision"))

(fn `UserConstructionScript`
  (bind _mesh (`self.Mesh`))
  (`SceneComponent.K2_AttachToComponent` (`self.LHandSphere`) _mesh "hand_l" "SnapToTarget" "SnapToTarget" "KeepWorld" true)
  (`SceneComponent.K2_AttachToComponent` (`self.RHandSphere`) _mesh "hand_r" "SnapToTarget" "SnapToTarget" "KeepWorld" true))